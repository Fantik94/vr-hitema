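; A breakable platform Blueprint that collapses when the ninja character touches it.
; On the first overlap of its capsule with BP_Ninja, it plays a wood-cracking sound at an arrow's location and turns on physics simulation for the static mesh.
; A DoOnce limits the collapse to a single trigger.
; BeginPlay stores the mesh's initial transform, which nothing in this graph uses afterward.
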(event `self.ReceiveBeginPlay`
  (set `self.TransformInit` (`SceneComponent.K2_GetComponentToWorld` (`self.StaticMesh`))))

(event `self.Capsule.OnComponentBeginOverlap`
  (params (OverlappedComponent :type "PrimitiveComponent Object Reference") (OtherActor :type "Actor Object Reference") (OtherComp :type "PrimitiveComponent Object Reference") (OtherBodyIndex :type Integer) (bFromSweep :type Boolean) (SweepResult :type "HitResult Structure (by ref)"))
  (bind _returnvalue_location (`KismetMathLibrary.BreakTransform` (`SceneComponent.K2_GetComponentToWorld` (`self.Arrow`))))
  (cast `/Game/personnages/BP_Ninja` OtherActor)
  (`/Engine/EditorBlueprintResources/StandardMacros.DoOnce` false
    (:`Completed`
      (`GameplayStatics.PlaySoundAtLocation` "/Game/Audio/wood-cracking.wood-cracking" _returnvalue_location (struct) 1.0 1.0 0.0 null null null null)
      (`PrimitiveComponent.SetSimulatePhysics` (`self.StaticMesh`) true))))

(fn `UserConstructionScript`)