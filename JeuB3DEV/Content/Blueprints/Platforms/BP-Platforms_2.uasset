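; BP-Platforms_2 is a falling platform that drops after BP_Ninja steps on it and then resets to its original position.
; BeginPlay stores the StaticMesh world transform.
; Overlapping the Capsule with the ninja starts a short delay before physics simulation is enabled on the mesh.
; After a further delay, RespawnPlatform disables physics and teleports the mesh back to the stored transform.
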(event `self.ReceiveBeginPlay`
  (set `self.TransformInit` (`SceneComponent.K2_GetComponentToWorld` (`self.StaticMesh`))))

(event `self.Capsule.OnComponentBeginOverlap`
  (params (OverlappedComponent :type "PrimitiveComponent Object Reference") (OtherActor :type "Actor Object Reference") (OtherComp :type "PrimitiveComponent Object Reference") (OtherBodyIndex :type Integer) (bFromSweep :type Boolean) (SweepResult :type "HitResult Structure (by ref)"))
  (cast `/Game/personnages/BP_Ninja` OtherActor)
  (`KismetSystemLibrary.Delay` 2.0)
  (`PrimitiveComponent.SetSimulatePhysics` (`self.StaticMesh`) true)
  (`KismetSystemLibrary.Delay` 5.0)
  (`self.RespawnPlatform`))

(event `RespawnPlatform`
  (bind _staticmesh (`self.StaticMesh`))
  (`PrimitiveComponent.SetSimulatePhysics` _staticmesh false)
  (`SceneComponent.K2_SetWorldTransform` _staticmesh (`self.TransformInit`) false true))

(fn `UserConstructionScript`)